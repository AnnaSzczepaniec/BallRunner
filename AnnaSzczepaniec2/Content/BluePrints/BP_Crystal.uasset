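; BP_Crystal is a pickup-style crystal that spins in yaw every Tick by a fixed, frame-rate-dependent step and is absorbed when the player touches it.
; On player overlap it disables the sphere's collision and caches its location, scale and light intensity.
; A timeline then lerps it toward the pawn's live position while shrinking it and fading the light, then destroys it.
; No reward is granted here.
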(event `self.ReceiveTick`
  (params (DeltaSeconds :type "Float (single-precision)"))
  (`self.ActorRotation`))

(event `self.Sphere.OnComponentBeginOverlap`
  (params (OverlappedComponent :type "PrimitiveComponent Object Reference") (OtherActor :type "Actor Object Reference") (OtherComp :type "PrimitiveComponent Object Reference") (OtherBodyIndex :type Integer) (bFromSweep :type Boolean) (SweepResult :type "HitResult Structure (by ref)"))
  (`/Game/Library/ML_ACTORS.IsPlayer` OtherActor
    (:`isPlayer?`
      (`PrimitiveComponent.SetCollisionEnabled` (`self.Sphere`) "NoCollision")
      (`self.CrystalPosition`)
      (`self.CrystalScale`)
      (`self.LerpIntensity`)
      (bind (_direction _location _scale _intensity) (`Timeline|TL_BlendAlfa`)
        (:`Update`
          (`self.CrystalToPawn` _location)
          (`self.Scale` _scale)
          (`self.Intensity` _intensity))
        (:`Finished`
          (`self.K2_DestroyActor`))))))

(fn `ActorRotation`
  (bind (_returnvalue_roll _returnvalue_pitch _returnvalue_yaw) (`KismetMathLibrary.BreakRotator` (`self.K2_GetActorRotation`)))
  (`self.K2_SetActorRotation` (`KismetMathLibrary.MakeRotator` _returnvalue_roll _returnvalue_pitch (+ _returnvalue_yaw 1.0))))

(fn `CrystalPosition`
  (set `self.LerpStartLocation` (`self.K2_GetActorLocation`)))

(fn `CrystalScale`
  (set `self.LerpStartScale` (`self.GetActorScale3D`)))

(fn `CrystalToPawn`
  (params (Alpha :type "Float (double-precision)"))
  (`self.K2_SetActorLocation` (`KismetMathLibrary.VLerp` (`self.LerpStartLocation`) (`self.K2_GetActorLocation` (`GameplayStatics.GetPlayerPawn` 0)) Alpha)))

(fn `Intensity`
  (params (Alpha :type "Float (double-precision)"))
  (`LightComponent.SetIntensity` (`self.PointLight`) (`KismetMathLibrary.Lerp` (`self.intensitylerp`) 0.0 Alpha)))

(fn `LerpIntensity`
  (set `self.intensitylerp` (`LightComponentBase.Intensity` (`self.PointLight`))))

(fn `Scale`
  (params (Alpha :type "Float (double-precision)"))
  (`self.SetActorScale3D` (`KismetMathLibrary.VLerp` (`self.LerpStartScale`) (0.0 0.0 0.0) Alpha)))

(fn `UserConstructionScript`)