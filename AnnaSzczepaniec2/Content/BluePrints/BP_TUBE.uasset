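; BP_TUBE is a tube actor that tracks when the player enters and leaves its overlap area.
; Begin and end overlap each check the other actor with IsPlayer, then cast player pawn 0 to BP_PAWN to set or clear a state flag on it.
; Leaving also resets the pawn's actor scale to its stored Scale value, while any behavior driven by the flag lives outside this Blueprint.
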(event `self.ReceiveActorEndOverlap`
  (params (OtherActor :type "Actor Object Reference"))
  (`/Game/Library/ML_ACTORS.IsPlayer` OtherActor
    (:`isPlayer?`
      (bind _asbp_pawn (cast `/Game/BluePrints/BP_PAWN` (`GameplayStatics.GetPlayerPawn` 0)))
      (set `/Game/BluePrints/BP_PAWN.IsPlayer...` false _asbp_pawn)
      (`self.SetActorScale3D` _asbp_pawn (`/Game/BluePrints/BP_PAWN.Scale` _asbp_pawn)))))

(event `self.ReceiveActorBeginOverlap`
  (params (OtherActor :type "Actor Object Reference"))
  (`/Game/Library/ML_ACTORS.IsPlayer` OtherActor
    (:`isPlayer?`
      (bind _asbp_pawn (cast `/Game/BluePrints/BP_PAWN` (`GameplayStatics.GetPlayerPawn` 0)))
      (set `/Game/BluePrints/BP_PAWN.IsPlayer...` true _asbp_pawn))))

(fn `UserConstructionScript`)