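; BP_Cannon is an automatic cannon that fires BP_Bullet projectiles repeatedly from the moment play begins.
; After a ProjectileTime delay, it spawns a bullet at the Arrow component's location and rotation, scaled by PorjectileScale.
; A timeline then animates the Cannon component's relative Y position as firing motion, and its Canon Fired event loops back to the delay for the next shot.
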(event `self.ReceiveBeginPlay`
  (`KismetSystemLibrary.Delay` (`self.Projectile Time`) :!label _label)
  (`self.SpawnProjectile`)
  (bind (_direction _time) (`Timeline|Canon Fire Timeline` :!via `PlayFromStart`)
    (:`Update`
      (`self.CanonPlacement` _time))
    (:`Canon Fired`
      (goto _label))))

(fn `CanonPlacement`
  (params (CanonBarrelY :type "Float (double-precision)"))
  (`SceneComponent.K2_SetRelativeLocation` (`self.Cannon`) (`KismetMathLibrary.MakeVector` 0.0 CanonBarrelY) false false))

(fn `SpawnProjectile`
  (bind (_returnvalue_location _returnvalue_rotation) (`KismetMathLibrary.BreakTransform` (`SceneComponent.K2_GetComponentToWorld` (`self.Arrow`))))
  (`|SpawnActorFromClass` "/Game/Projectiles/BP_Bullet.BP_Bullet_C" (`KismetMathLibrary.MakeTransform` _returnvalue_location _returnvalue_rotation (`KismetMathLibrary.Conv_DoubleToVector` (`self.Porjectile Scale`))) "Undefined" "OverrideRootScale" null null))

(fn `UserConstructionScript`)