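; Player pawn rolled as a physics sphere by applying torque from the UpDown and RightLeft input axes.
; Holding right mouse shrinks it to half scale, and releasing restores the scale saved at BeginPlay only when an IsPlayer check is false, with debug prints.
; Any damage triggers Death, which fades the camera and reloads the current level after a delay, while Escape quits the game.
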(event `Key|Escape`
  (params (Key :type "Key Structure"))
  (:`Pressed`
    (`KismetSystemLibrary.QuitGame` null "Quit")))

(event `InputAxis|UpDown`
  (params (AxisValue :type "Float (single-precision)"))
  (`PrimitiveComponent.AddTorqueInRadians` (`self.Sphere`) (`KismetMathLibrary.MakeVector` (* (stale `InputAxis|RightLeft` AxisValue) (`self.multiply`)) (* AxisValue (`self.multiply`))) "None" true :!label _label))

(event `InputAxis|RightLeft`
  (params (AxisValue :type "Float (single-precision)"))
  (goto _label))

(event `self.ReceiveAnyDamage`
  (params (Damage :type "Float (single-precision)") (DamageType :type "DamageType Object Reference") (InstigatedBy :type "Controller Object Reference") (DamageCauser :type "Actor Object Reference"))
  (`self.Death`))

(event `self.ReceiveBeginPlay`
  (set `self.Scale` (`self.GetActorScale3D`)))

(event `Key|RightMouseButton`
  (params (Key :type "Key Structure"))
  (:`Pressed`
    (`self.SetActorScale3D` (0.5 0.5 0.5)))
  (:`Released`
    (if (`self.IsPlayer...`)
      (`KismetSystemLibrary.PrintString` "true")
      (else
        (`KismetSystemLibrary.PrintString` "false")
        (`self.SetActorScale3D` (`self.Scale`))))))

(fn `UserConstructionScript`)