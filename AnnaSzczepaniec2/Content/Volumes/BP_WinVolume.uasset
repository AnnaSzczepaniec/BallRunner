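; BP_WinVolume is a level-exit trigger that completes the level when the player overlaps it with no BP_Crystal actors left in the world.
; It looks up the current level in the ordered LevelName array and opens the following entry, or quits the game on the last one.
; The crystal check is evaluated only when an overlap begins, by counting all remaining crystal actors.
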(event `self.ReceiveActorBeginOverlap`
  (params (OtherActor :type "Actor Object Reference"))
  (`/Game/Library/ML_ACTORS.IsPlayer` OtherActor
    (:`isPlayer?`
      (if (`self.CheckAnyCrystal`)
        (`self.CompleteLevel`)))))

(fn `CheckAnyCrystal`
  (returns (ReturnValue :type Boolean))
  (bind _outactors (`GameplayStatics.GetAllActorsOfClass` "/Game/BluePrints/BP_Crystal.BP_Crystal_C"))
  (return (== (`KismetArrayLibrary.Array_Length` _outactors) 0)))

(fn `CompleteLevel`
  (if (`self.IsFinalLevel`)
    (`KismetSystemLibrary.QuitGame` null "Quit")
    (else
      (`GameplayStatics.OpenLevel` (`self.GetNextLevelName`)))))

(fn `GetCurrentLevelIndex`
  (returns (IndexNumber :type Integer))
  (bind _returnvalue (`GameplayStatics.GetCurrentLevelName` true))
  (return (`KismetArrayLibrary.Array_Find` (`self.LevelName`) (`KismetStringLibrary.Conv_StringToName` _returnvalue))))

(fn `GetLastLevelIndex`
  (returns (ReturnValue :type Integer))
  (return (`KismetArrayLibrary.Array_LastIndex` (`self.LevelName`))))

(fn `GetNextLevelName`
  (returns (Output :type "Name (by ref)"))
  (bind _returnvalue (`GameplayStatics.GetCurrentLevelName` true))
  (return (`|GetArrayItem` (`self.LevelName`) (+ (`KismetArrayLibrary.Array_Find` (`self.LevelName`) (`KismetStringLibrary.Conv_StringToName` _returnvalue)) 1))))

(fn `IsFinalLevel`
  (returns (ReturnValue :type Boolean))
  (return (== (`self.GetLastLevelIndex`) (`self.GetCurrentLevelIndex`))))

(fn `UserConstructionScript`)